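; BP_NPC is a wandering NPC Blueprint that roams to random reachable points around its current location.
; Each tick passes a DoOnce gate to start an AI MoveTo, with the gate resetting one second after a successful move; a failed move never resets it.
; Pawn Sensing stores any seen BP_Player in a Player variable, which these graphs do not otherwise use.
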(event `self.ReceiveTick`
  (params (DeltaSeconds :type "Float (single-precision)"))
  (`|ExecutionSequence`
    (:`then_0`
      (`/Engine/EditorBlueprintResources/StandardMacros.DoOnce` false :!label _label
        (:`Completed`
          (bind _randompoint (`self.GetRandomLocation`))
          (`|AIMoveTo` self _randompoint null
            (:`OnSuccess`
              (`KismetSystemLibrary.Delay` 1.0)
              (goto _label :!via `Reset`))))))))

(event `self.PawnSensing.OnSeePawn`
  (params (Pawn :type "Pawn Object Reference"))
  (bind _asbp_player (cast `/Game/Character/Blueprints/BP_Player` Pawn))
  (set `self.Player` _asbp_player))

(fn `GetRandomLocation`
  (returns (RandomPoint :type "Vector Structure"))
  (bind _output_get (set `self.Random Location_0` (`NavigationSystemV1.K2_GetRandomReachablePointInRadius` (`self.K2_GetActorLocation`) (`self.Radius`) null null)))
  (return _output_get))

(fn `UserConstructionScript`
  (`parent.UserConstructionScript`))