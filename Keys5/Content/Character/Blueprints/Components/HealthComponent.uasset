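; HealthComponent is an actor component that tracks health for a BP_Character and handles its death.
; BeginPlay caches the owning character and fills health to max, and ChangeHealth subtracts damage without clamping.
; Tick polls Dead every frame; at zero health or below it repeatedly sets the dead flag, disables movement, player 0 input and capsule collision, and turns the mesh into a physics ragdoll.
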(event `self.ReceiveBeginPlay`
  (bind _asbp_character (cast `/Game/Character/Blueprints/BP_Character` (`self.GetOwner`)))
  (set `self.Character` _asbp_character)
  (set `self.Health` (`self.HealthMax`)))

(event `self.ReceiveTick`
  (params (DeltaSeconds :type "Float (single-precision)"))
  (`self.Dead`))

(fn `ChangeHealth`
  (params (Damage :type "Float (double-precision)"))
  (set `self.Health` (- (`self.Health`) Damage)))

(fn `Dead`
  (bind _mesh (`Character.Mesh` (`self.Character`)))
  (if (not (> (`self.Health`) 0.0))
    (set `self.Dead?` true)
    (`CharacterMovementComponent.DisableMovement` (`Character.CharacterMovement` (`self.Character`)))
    (`Actor.DisableInput` (`self.Character`) (`GameplayStatics.GetPlayerController` 0))
    (`PrimitiveComponent.SetCollisionEnabled` (`Character.CapsuleComponent` (`self.Character`)) "NoCollision")
    (`PrimitiveComponent.SetCollisionEnabled` _mesh "QueryAndPhysics")
    (`PrimitiveComponent.SetSimulatePhysics` _mesh true)))