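; Melee enemy NPC that chases the player and punches on reaching them.
; Each tick it issues AI MoveTo toward a valid, living Player; success triggers Hit.
; Hit uses a DoOnce to play a boxing animation, pulse the Attack flag on timed delays, and pause tick and pawn sensing until finished.
; Hand overlaps apply BaseDamage to BP_Player without checking Attack in this graph.
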(event `self.ReceiveTick`
  (params (DeltaSeconds :type "Float (single-precision)"))
  (bind _player (`self.Player`))
  (`parent.ReceiveTick` DeltaSeconds)
  (`/Engine/EditorBlueprintResources/StandardMacros.IsValid` _player
    (:`Is Valid`
      (if (not (`/Game/Character/Blueprints/Components/HealthComponent.Dead?` (`/Game/Character/Blueprints/BP_Player.HealthComponent` _player)))
        (`|AIMoveTo` self (0.0 0.0 0.0) _player
          (:`OnSuccess`
            (`self.Hit`)))))))

(event `Hit`
  (`/Engine/EditorBlueprintResources/StandardMacros.DoOnce` false :!label _label
    (:`Completed`
      (`self.StopForHit` true)
      (`SkeletalMeshComponent.PlayAnimation` (`self.Mesh`) "/Game/Character/Animations/Boxing.Boxing" false)
      (`KismetSystemLibrary.Delay` 0.5)
      (set `self.Attack` true)
      (`KismetSystemLibrary.Delay` 0.4)
      (set `self.Attack` false)
      (`KismetSystemLibrary.Delay` 1.2)
      (`SkeletalMeshComponent.SetAnimationMode` (`self.Mesh`) "AnimationBlueprint" true)
      (`self.StopForHit` false)
      (goto _label :!via `Reset`))))

(event `self.Hand.OnComponentBeginOverlap`
  (params (OverlappedComponent :type "PrimitiveComponent Object Reference") (OtherActor :type "Actor Object Reference") (OtherComp :type "PrimitiveComponent Object Reference") (OtherBodyIndex :type Integer) (bFromSweep :type Boolean) (SweepResult :type "HitResult Structure (by ref)"))
  (bind _asbp_player (cast `/Game/Character/Blueprints/BP_Player` OtherActor))
  (`GameplayStatics.ApplyDamage` _asbp_player (`self.Base Damage`)))

(fn `StopForHit`
  (params (Stop :type Boolean))
  (bind _pawnsensing (`self.PawnSensing`))
  (if Stop
    (`self.SetActorTickEnabled` false)
    (`PawnSensingComponent.SetSensingUpdatesEnabled` _pawnsensing false)
    (else
      (`self.SetActorTickEnabled` true)
      (`PawnSensingComponent.SetSensingUpdatesEnabled` _pawnsensing true))))

(fn `UserConstructionScript`
  (`parent.UserConstructionScript`))